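; HUD for the BGE game that creates the main UI widget and drives the flow from countdown through gameplay to game end.
; StartCountdown applies the chosen vehicle data to the BGE pawn, locks its input and starts a looping one-second timer.
; When the counter hits zero, StartGame restores input and shows the in-game view.
; Each phase, including EndGame, switches pages on the UI's widget switcher.
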(event `self.ReceiveBeginPlay`
  (bind _returnvalue (`|CreateWidget` "/Game/BestGameEver/Core/Game/WBP_UI.WBP_UI_C" (`self.GetOwningPlayerController`)))
  (bind _output_get (set `self.UI` _returnvalue))
  (bind _output_get_2 (set `/Game/BestGameEver/Core/Game/WBP_UI.HUD` self _output_get))
  (set `/Game/BestGameEver/Core/Game/WBP_Countdown.HUD` _output_get_2 (`/Game/BestGameEver/Core/Game/WBP_UI.WBP_Countdown` _output_get))
  (`UserWidget.AddToPlayerScreen` _output_get 0))

(event `StartCountdown`
  (params (VehicleData :type "/Game/BestGameEver/Core/Player/Vehicle Structure"))
  (bind _ui (`self.UI`))
  (`WidgetSwitcher.SetActiveWidgetIndex` (`/Game/BestGameEver/Core/Game/WBP_UI.WidgetSwitcher_164` _ui) 1)
  (`/Game/BestGameEver/Core/Game/WBP_Countdown.StartBlurFadeIn` (`/Game/BestGameEver/Core/Game/WBP_UI.WBP_Countdown` _ui))
  (bind _asbp_bgepawn (cast `/Game/BestGameEver/Core/Player/BP_BGEPawn` (`self.GetOwningPawn`)))
  (`/Game/BestGameEver/Core/Player/BP_BGEPawn.SetVehicle` _asbp_bgepawn VehicleData)
  (`self.DisableInput` _asbp_bgepawn (`self.GetOwningPlayerController`))
  (set `/Game/BestGameEver/Core/Game/WBP_InGame.Pawn` _asbp_bgepawn (`/Game/BestGameEver/Core/Game/WBP_UI.WBP_InGame` _ui))
  (`KismetSystemLibrary.K2_SetTimerDelegate` (delegate `Countdown`) 1.0 true))

(event `Countdown`
  (bind _output_get (set `self.Counter` (- (`self.Counter`) 1)))
  (if (== _output_get 0)
    (`self.StartGame`)))

(event `StartGame`
  (bind _asbp_bgepawn (cast `/Game/BestGameEver/Core/Player/BP_BGEPawn` (`self.GetOwningPawn`)))
  (`self.EnableInput` _asbp_bgepawn (`self.GetOwningPlayerController`))
  (`WidgetSwitcher.SetActiveWidgetIndex` (`/Game/BestGameEver/Core/Game/WBP_UI.WidgetSwitcher_164` (`self.UI`)) 2))

(event `EndGame`
  (`WidgetSwitcher.SetActiveWidgetIndex` (`/Game/BestGameEver/Core/Game/WBP_UI.WidgetSwitcher_164` (`self.UI`)) 3))

(fn `UserConstructionScript`)