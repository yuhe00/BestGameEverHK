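; BP_Rocket is a rocket projectile that flies straight ahead and explodes when its movement fails.
; Each Tick it moves along its forward vector at Speed, scaled by delta time, using a swept SetActorLocation instead of physics.
; When that move returns false, it creates an explosion at the impact point and destroys itself.
; If the hit actor is a BP_Rock, it calls that rock's Destroy with the impact point and normal.
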(event `self.ReceiveTick`
  (params (DeltaSeconds :type "Float (single-precision)"))
  (bind (_sweephitresult _returnvalue) (`self.K2_SetActorLocation` (+ (`self.K2_GetActorLocation`) (* (`self.GetActorForwardVector`) (* DeltaSeconds (`self.Speed`)))) true))
  (if (not _returnvalue)
    (bind (_bblockinghit _binitialoverlap _time _distance _location _impactpoint _normal _impactnormal _physmat _hitactor) (`GameplayStatics.BreakHitResult` _sweephitresult))
    (`/Game/BestGameEver/Core/Rocket/BP_Explode.CreateExplosion` _impactpoint)
    (`self.K2_DestroyActor`)
    (bind _asbp_rock (cast `/Game/BestGameEver/Core/Rock/BP_Rock` _hitactor))
    (`/Game/BestGameEver/Core/Rock/BP_Rock.Destroy` _asbp_rock _impactpoint _impactnormal)))

(fn `UserConstructionScript`)